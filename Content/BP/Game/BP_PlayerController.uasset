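; Player controller for an Open World Server (OWS) game that owns the client HUD, inventory menu toggle, interact input and floating damage text.
; Remote clients create the HUD widgets on BeginPlay, binding some to BagInventory, then fill the name plate and hide loading when ready.
; Client Tick polls GAS combat attributes for health and a three-segment stamina bar.
; Serialized base character stats persist as OWS custom character data.
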(event Custom|PersistBaseCharacterStats
  (bind _returnvalue (Class|HWCharacter|SerializeBaseCharacterStats (Class|HWPlayerController|GetHWGASPlayerCharacter)))
  (Class|OWSPlayerControllerComponent|AddorUpdateCustomCharacterData (Variables|Default|GetOWSPlayerControllerComponent) (PlayerState|GetPlayerName (Class|OWSPlayerControllerComponent|GetOWSPlayerState (Variables|Default|GetOWSPlayerControllerComponent))) "BaseCharacterStats" _returnvalue))

(event EventBeginPlay
  (Networking|SwitchHasAuthority
    (:Remote
      (CallFunction|SetupHUD))))

(event EventTick
  (params (DeltaSeconds :type Float%20%28single-precision%29))
  (bind _resourcebarshudwidget (Variables|Default|GetResourceBarsHUDWidget))
  (bind _resourcebarshudwidget_2 (Variables|Default|GetResourceBarsHUDWidget))
  (Networking|SwitchHasAuthority
    (:Remote
      (bind _ashwgasplayer_character (Utilities|Casting|CastToHWGASPlayerCharacter (Pawn|GetControlledPawn)))
      (bind _returnvalue (GameplayAttributes|GetAttributeSet (Variables|/Script/OWSHubWorldMMO.HWGASCharacter|GetAbilitySystem _ashwgasplayer_character) "/Script/OWSHubWorldMMO.HWCombatAttributeSet"))
      (bind _ashwcombat_attribute_set (Utilities|Casting|CastToHWCombatAttributeSet _returnvalue))
      (if (> (Class|HWCombatAttributeSet|HWGetMaxHealth _ashwcombat_attribute_set) 0.0)
        (if (Utilities|IsValid _resourcebarshudwidget_2)
          (Progress|SetPercent (Variables|/Game/BP/HUD/ResourceBarsHUDWidget.ResourceBarsHUDWidget_C|GetHPBar _resourcebarshudwidget_2) (Math|Float|Clamp(Float) (/ (Class|HWCombatAttributeSet|HWGetHealth _ashwcombat_attribute_set) (Class|HWCombatAttributeSet|HWGetMaxHealth _ashwcombat_attribute_set))))
          (Progress|SetPercent (Variables|/Game/BP/HUD/ResourceBarsHUDWidget.ResourceBarsHUDWidget_C|GetStaminaBarPart1 _resourcebarshudwidget) (Math|Float|Clamp(Float) (/ (Math|Float|Clamp(Float) (/ (Class|HWCombatAttributeSet|HWGetStamina _ashwcombat_attribute_set) (Class|HWCombatAttributeSet|HWGetMaxStamina _ashwcombat_attribute_set))) 0.33)))
          (Progress|SetPercent (Variables|/Game/BP/HUD/ResourceBarsHUDWidget.ResourceBarsHUDWidget_C|GetStaminaBarPart2 _resourcebarshudwidget) (Math|Float|Clamp(Float) (/ (Math|Float|Clamp(Float) (- (Math|Float|Clamp(Float) (/ (Class|HWCombatAttributeSet|HWGetStamina _ashwcombat_attribute_set) (Class|HWCombatAttributeSet|HWGetMaxStamina _ashwcombat_attribute_set))) 0.33)) 0.33)))
          (Progress|SetPercent (Variables|/Game/BP/HUD/ResourceBarsHUDWidget.ResourceBarsHUDWidget_C|GetStaminaBarPart3 _resourcebarshudwidget) (Math|Float|Clamp(Float) (/ (Math|Float|Clamp(Float) (- (Math|Float|Clamp(Float) (/ (Class|HWCombatAttributeSet|HWGetStamina _ashwcombat_attribute_set) (Class|HWCombatAttributeSet|HWGetMaxStamina _ashwcombat_attribute_set))) 0.66)) 0.33))))))))

(event EventReadytoPlayonServer)

(event EventReadytoPlayonClient
  (Variables|/Script/UMG.TextBlock|SetText (Variables|/Game/BP/HUD/PlayerNamePlateWidget.PlayerNamePlateWidget_C|GettxtPlayerName (Variables|Default|GetPlayerNamePlateWidget)) (Utilities|Text|ToText(String) (PlayerState|GetPlayerName (Class|HWPlayerController|GetOWSPlayerState))))
  (bind _asbp_hub_world_game_instance (Utilities|Casting|CastToBP_HubWorldGameInstance (Game|GetGameInstance)))
  (Class|OWSGameInstance|HideLoadingScreen _asbp_hub_world_game_instance))

(event Input|EnhancedActionEvents|EnhancedInputActionIA_OpenMenu
  (params (ActionValue :type Boolean) (ElapsedSeconds :type Float%20%28double-precision%29) (TriggeredSeconds :type Float%20%28double-precision%29) (InputAction :type Input%20Action%20Object%20Reference :default "/Game/Input/Actions/IA_OpenMenu.IA_OpenMenu"))
  (bind _self self)
  (bind _riftinventory (Variables|Default|GetRiftInventory))
  (:Started
    (Utilities|FlowControl|FlipFlop
      (:A
        (UserInterface|Viewport|AddtoViewport _riftinventory 0)
        (Development|PrintString "Show Inventory")
        (Input|SetInputModeGameandUI _self 0 "DoNotLock" true false)
        (Variables|Default|SetbShowMouseCursor true))
      (:B
        (Widget|RemovefromParent _riftinventory)
        (Input|SetInputModeGameOnly _self false)
        (Variables|Default|SetbShowMouseCursor false)))))

(event Input|EnhancedActionEvents|EnhancedInputActionIA_Interact
  (params (ActionValue :type Boolean) (ElapsedSeconds :type Float%20%28double-precision%29) (TriggeredSeconds :type Float%20%28double-precision%29) (InputAction :type Input%20Action%20Object%20Reference :default "/Game/Input/Actions/IA_Interact.IA_Interact"))
  (:Started
    (Class|HWPlayerController|Interact)))

(fn ConstructionScript)

(fn SetupHUD
  (Utilities|FlowControl|Sequence
    (:then_0
      (bind _returnvalue (UserInterface|CreateWidget "/Game/BP/HUD/ResourceBarsHUDWidget.ResourceBarsHUDWidget_C" self))
      (bind _output_get (Variables|Default|SetResourceBarsHUDWidget _returnvalue))
      (UserInterface|Viewport|AddtoViewport _output_get 0))
    (:then_1
      (bind _returnvalue_2 (UserInterface|CreateWidget "/Game/BP/CommonUI/BaseUI.BaseUI_C" self))
      (bind _output_get_2 (Variables|Default|SetBaseUIWidget _returnvalue_2))
      (UserInterface|Viewport|AddtoViewport _output_get_2 0))
    (:then_2
      (Variables|Default|SetInventoryComponentForInventoryUI (Variables|Default|GetBagInventory)))
    (:then_3
      (bind _returnvalue_3 (UserInterface|CreateWidget "/Game/BP/Inventory/UI/CommonInventoryListWidget.CommonInventoryListWidget_C" self))
      (bind _output_get_3 (Variables|Default|SetCommonInventoryListWidget _returnvalue_3))
      (Class|HWCommonInventoryListWidget|SetInventoryComponent _output_get_3 (Variables|Default|GetBagInventory)))
    (:then_4
      (bind _returnvalue_4 (UserInterface|CreateWidget "/Game/BP/CommonUI/MenuTabs.MenuTabs_C" self))
      (bind _output_get_4 (Variables|Default|SetMenuTabsWidget _returnvalue_4))
      (Class|HWCommonInventoryListWidget|SetInventoryComponent (Variables|/Game/BP/CommonUI/InventoryTab.InventoryTab_C|GetCommonInventoryListWidget (Variables|/Game/BP/CommonUI/MenuTabs.MenuTabs_C|GetInventoryTab _output_get_4)) (Variables|Default|GetBagInventory)))
    (:then_5
      (bind _returnvalue_5 (UserInterface|CreateWidget "/Game/BP/HUD/AbilityCooldownsWidget.AbilityCooldownsWidget_C" self))
      (bind _output_get_5 (Variables|Default|SetAbilityCooldownsWidget _returnvalue_5))
      (UserInterface|Viewport|AddtoViewport _output_get_5 0))
    (:then_6
      (bind _returnvalue_6 (UserInterface|CreateWidget "/Game/BP/HUD/PlayerNamePlateWidget.PlayerNamePlateWidget_C" self))
      (bind _output_get_6 (Variables|Default|SetPlayerNamePlateWidget _returnvalue_6))
      (UserInterface|Viewport|AddtoViewport _output_get_6 0))
    (:then_7
      (bind _returnvalue_7 (UserInterface|CreateWidget "/Game/BP/Inventory/RiftUI/WBP_Inventory.WBP_Inventory_C" self))
      (Variables|Default|SetRiftInventory _returnvalue_7))))

(fn AddFloatingDamage
  (params (DamageText :type String) (DamagedActor :type Actor%20Object%20Reference) (IsCritical :type Boolean))
  (bind _asbp_hud (Utilities|Casting|CastToBP_HUD (HUD|GetHUD)))
  (Class|HWHUD|AddFloatingDamageItem _asbp_hud DamageText DamagedActor (Math|Vector2D|MakeVector2D (Math|Random|RandomFloatinRange -2e+02 2e+02) (Math|Random|RandomFloatinRange -1.8e+02 -9e+01)) false IsCritical true false))