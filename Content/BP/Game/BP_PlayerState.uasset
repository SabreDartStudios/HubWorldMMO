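; Player state Blueprint that smoke-tests the Rift inventory component with debug prints.
; On BeginPlay, the authority waits for inventory initialization, then adds a test item to the Backpack container and prints the result.
; Both authority and remote print the Backpack item count after a short fixed delay, independent of the initialization callback.
; GetInventoryComponent is an empty stub.
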(event Custom|InventoryInitialized
  (params (bSuccess :type Boolean))
  (bind _inventorycomponent (Variables|Default|GetInventoryComponent))
  (Development|PrintString "Rift: Initialized")
  (if bSuccess
    (bind _returnvalue (Class|RiftInventoryComponent|AddItemtoContainer _inventorycomponent "/Game/BP/Inventory/Items/DA_Item_Test.DA_Item_Test" (Class|RiftInventoryComponent|GetContainerbyTag _inventorycomponent "(TagName=\"Rift.Container.Backpack\")") 1))
    (Development|PrintString (Utilities|String|Append "Rift: " (Guid|ToString(Guid) _returnvalue)))
    (else
      (Development|PrintString "Rift Inventory Not Initialized"))))

(event EventBeginPlay
  (bind _inventorycomponent (Variables|Default|GetInventoryComponent))
  (Networking|SwitchHasAuthority
    (:Authority
      (Development|PrintString "Rift: Start waiting for initialized")
      (Class|RiftInventoryComponent|WaitforInitialized _inventorycomponent (delegate Custom|InventoryInitialized)))
    (:Remote
      _))
  (Utilities|FlowControl|Delay 2.0)
  (Development|PrintString (Utilities|String|Append "Rift: " (Utilities|String|ToString(Integer) (Utilities|Array|Length (Class|RiftContainer|GetAllItems (Class|RiftInventoryComponent|GetContainerbyTag _inventorycomponent "(TagName=\"Rift.Container.Backpack\")")))))))

(event EventTick
  (params (DeltaSeconds :type Float%20%28single-precision%29)))

(fn ConstructionScript)

(fn GetInventoryComponent
  (return 0))