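; Player controller for the login screen, running the OWS flow from login and registration through character creation to connecting to the game.
; BeginPlay sets a camera actor as view target and creates all dialog widgets, which show/hide functions swap.
; OWS component callbacks load the first character into the detail dialog, or open creation if none exists; connecting joins its last zone.
; Tick slowly lowers the directional light's pitch toward -20 degrees as backdrop animation.
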(event EventBeginPlay
  (|CallParentFunction)
  (bind _outactors (Actor|GetAllActorsOfClass "/Script/Engine.CameraActor"))
  (Game|Player|SetViewTargetwithBlend (Utilities|Array|Get(acopy) _outactors) 0.0 "VTBlend_Linear" 0.0 false)
  (bind _outactors_2 (Actor|GetAllActorsOfClass "/Script/Engine.DirectionalLight"))
  (Variables|Default|SetSunLight (Utilities|Array|Get(acopy) _outactors_2))
  (Dialogs|SetupDialogs)
  (Dialogs|ShowLoginDialog)
  (Input|SetInputModeUIOnly self (Variables|Widgets|GetUILoginWidget) "DoNotLock" false))

(event EventTick
  (params (DeltaSeconds :type Float%20%28single-precision%29))
  (bind _sunlight (Variables|Default|GetSunLight))
  (bind _returnvalue (Transformation|GetActorRotation _sunlight))
  (|CallParentFunction DeltaSeconds)
  (if (!= _sunlight 0)
    (if (> (.pitch _returnvalue) -2e+01)
      (Transformation|SetActorRotation _sunlight (Math|Rotator|MakeRotator (.roll _returnvalue) (+ (.pitch _returnvalue) -0.001) (.yaw _returnvalue))))))

(event EventNotifyCreateCharacterUsingDefaultCharacterValues
  (Dialogs|HideCreateCharacter)
  (Dialogs|ShowCharacterDetailDialog))

(event EventErrorGetAllCharacters
  (params (ErrorMsg :type String))
  (Development|PrintString ErrorMsg))

(event EventNotifyGetAllCharacters
  (params (UserCharacters :type Array%20of%20User%20Character%20Structures))
  ;[1 1 1] Get the Character associated with the logged in User
  (if (> (Utilities|Array|Length UserCharacters) 0)
    (CallFunction|GetFirstCharacterData UserCharacters)
    (Class|OWSPlayerControllerComponent|GetCharacterDataandCustomData (Variables|Default|GetOWSPlayerControllerComponent) (Variables|Default|GetUserSessionGUID) (Variables|Default|GetCharacterName))
    (else
      (Dialogs|ShowCreateCharacterDialog))))

(event EventErrorCreateCharacterUsingDefaultCharacterValues
  (params (ErrorMsg :type String))
  (Dialogs|ShowCreateCharacterDialog ErrorMsg))

(event EventNotifyGetCharacterDataandCustomData
  (params (CustomCharacterData :type Array%20of%20Custom%20Character%20Data%20Struct%20Structures))
  (for _array_element CustomCharacterData
    (if (Utilities|Enum|Equal(Enum) (.CustomFieldName (Utilities|Struct|BreakCustomCharacterDataStruct _array_element)) "CosmeticCharacterData")
      (Development|PrintString (.FieldValue (Utilities|Struct|BreakCustomCharacterDataStruct _array_element)))
      (elif (Utilities|Enum|Equal(Enum) (.CustomFieldName (Utilities|Struct|BreakCustomCharacterDataStruct _array_element)) "ReadOnlyCharacterData")
        (Development|PrintString (.FieldValue (Utilities|Struct|BreakCustomCharacterDataStruct _array_element))))))
  (Dialogs|ShowCharacterDetailDialog))

(fn ConstructionScript
  (|CallParentFunction))

(fn ShowLoadingDialog
  (bind _uifullscreenloadingwidget (Variables|Widgets|GetUIFullScreenLoadingWidget))
  (Default|PlayFadein _uifullscreenloadingwidget)
  (UserInterface|Viewport|AddtoViewport _uifullscreenloadingwidget 0))

(fn HideLoadingDialog
  (bind _uifullscreenloadingwidget (Variables|Widgets|GetUIFullScreenLoadingWidget))
  (Default|PlayFadeOut _uifullscreenloadingwidget)
  (Widget|RemovefromParent _uifullscreenloadingwidget))

(fn HideLoginDialog
  (bind _uiloginwidget (Variables|Widgets|GetUILoginWidget))
  (Default|PlayFadeOut _uiloginwidget)
  (Widget|RemovefromParent _uiloginwidget))

(fn SetupDialogs
  (bind _returnvalue (UserInterface|CreateWidget "/Game/BP/Login/UI_LoginWidget.UI_LoginWidget_C"))
  (Variables|Widgets|SetUILoginWidget _returnvalue)
  (bind _returnvalue_2 (UserInterface|CreateWidget "/Game/BP/Login/UI_RegisterWidget.UI_RegisterWidget_C"))
  (Variables|Widgets|SetUIRegisterWidget _returnvalue_2)
  (bind _returnvalue_3 (UserInterface|CreateWidget "/Game/BP/Login/UI_FullScreenLoadingDialog.UI_FullScreenLoadingDialog_C"))
  (Variables|Widgets|SetUIFullScreenLoadingWidget _returnvalue_3)
  (bind _returnvalue_4 (UserInterface|CreateWidget "/Game/BP/Login/UI_CreateCharacterWidget.UI_CreateCharacterWidget_C"))
  (Variables|Widgets|SetUICreateCharacter _returnvalue_4)
  (bind _returnvalue_5 (UserInterface|CreateWidget "/Game/BP/Login/UI_MessageConfirmWidget.UI_MessageConfirmWidget_C"))
  (Variables|Widgets|SetUIMessageConfirm _returnvalue_5)
  (bind _returnvalue_6 (UserInterface|CreateWidget "/Game/BP/Login/UI_CharacterDetailWidget.UI_CharacterDetailWidget_C"))
  (Variables|Widgets|SetUICharacterDetailWidget _returnvalue_6))

(fn ShowRegisterDialog
  (bind _uiregisterwidget (Variables|Widgets|GetUIRegisterWidget))
  (Widget|RemovefromParent (Variables|Widgets|GetUILoginWidget))
  (Default|PlayFadein _uiregisterwidget)
  (UserInterface|Viewport|AddtoViewport _uiregisterwidget 0)
  (Widget|SetFocus (Variables|/Game/BP/Login/UI_RegisterWidget.UI_RegisterWidget_C|GettxtFirstName _uiregisterwidget)))

(fn LoginComplete
  (params (UserSessionGUID :type String))
  (Variables|Default|SetUserSessionGUID UserSessionGUID)
  (Dialogs|HideLoginDialog)
  (Dialogs|HideLoadingDialog)
  (Class|OWSPlayerControllerComponent|GetAllCharacters (Variables|Default|GetOWSPlayerControllerComponent) (Variables|Default|GetUserSessionGUID)))

(fn GetFirstCharacterData
  (params (UserCharacters :type Array%20of%20User%20Character%20Structures))
  (Variables|Default|SetCharacterName (.CharacterName (Utilities|Struct|BreakUserCharacter (Utilities|Array|Get(acopy) UserCharacters)))))

(fn HideRegisterDialog
  (bind _uiregisterwidget (Variables|Widgets|GetUIRegisterWidget))
  (Default|PlayFadeOut _uiregisterwidget)
  (Widget|RemovefromParent _uiregisterwidget))

(fn ShowLoginDialog
  (bind _uiloginwidget (Variables|Widgets|GetUILoginWidget))
  (Default|PlayFadein _uiloginwidget)
  (UserInterface|Viewport|AddtoViewport _uiloginwidget 0)
  (Rendering|Components|TextRender|SetText (Variables|/Game/BP/Login/UI_LoginWidget.UI_LoginWidget_C|GettxtPassword _uiloginwidget) "")
  (Widget|SetFocus (Variables|/Game/BP/Login/UI_LoginWidget.UI_LoginWidget_C|GettxtEmail _uiloginwidget)))

(fn ShowCreateCharacterDialog
  (params (InitialCreateCharacterMessage :type String))
  (bind _uicreatecharacter (Variables|Widgets|GetUICreateCharacter))
  (bind _txtcharactername (Variables|/Game/BP/Login/UI_CreateCharacterWidget.UI_CreateCharacterWidget_C|GettxtCharacterName _uicreatecharacter))
  (UserInterface|Viewport|AddtoViewport _uicreatecharacter 0)
  (Rendering|Components|TextRender|SetText _txtcharactername "")
  (Widget|SetFocus _txtcharactername)
  (Widget|SetIsEnabled (Variables|/Game/BP/Login/UI_CreateCharacterWidget.UI_CreateCharacterWidget_C|GetbtnContinue _uicreatecharacter) false)
  (if (not (Utilities|Array|IsEmpty InitialCreateCharacterMessage))
    (Rendering|Components|TextRender|SetText (Variables|/Game/BP/Login/UI_CreateCharacterWidget.UI_CreateCharacterWidget_C|GetlitCreateCharacterMessage _uicreatecharacter) (Utilities|Text|ToText(String) InitialCreateCharacterMessage))))

(fn HideCreateCharacter
  (Widget|RemovefromParent (Variables|Widgets|GetUICreateCharacter)))

(fn CreateCharacter
  (params (CharacterName :type String))
  (Class|OWSPlayerControllerComponent|CreateCharacter (Variables|Default|GetOWSPlayerControllerComponent) (Variables|Default|GetUserSessionGUID) CharacterName (Variables|Default|GetDefaultClassName)))

(fn ShowMessageConfirmDialog
  (params (MessageText :type String))
  (bind _uimessageconfirm (Variables|Widgets|GetUIMessageConfirm))
  (Variables|/Script/UMG.TextBlock|SetText (Variables|/Game/BP/Login/UI_MessageConfirmWidget.UI_MessageConfirmWidget_C|GettxtMessageText _uimessageconfirm) (Utilities|Text|ToText(String) MessageText))
  (UserInterface|Viewport|AddtoViewport _uimessageconfirm 0))

(fn HideMessageConfirmDialog
  (Widget|RemovefromParent (Variables|Widgets|GetUIMessageConfirm)))

(fn ShowCharacterDetailDialog
  (bind _uicharacterdetailwidget (Variables|Widgets|GetUICharacterDetailWidget))
  (Variables|/Script/UMG.TextBlock|SetText (Variables|/Game/BP/Login/UI_CharacterDetailWidget.UI_CharacterDetailWidget_C|GettxtCharacterName _uicharacterdetailwidget) (Utilities|Text|ToText(String) (Variables|Default|GetCharacterName)))
  (Default|PlayFadein _uicharacterdetailwidget)
  (UserInterface|Viewport|AddtoViewport _uicharacterdetailwidget 0))

(fn HideCharacterDetailDialog
  (bind _uicharacterdetailwidget (Variables|Widgets|GetUICharacterDetailWidget))
  (Default|PlayFadeOut _uicharacterdetailwidget)
  (Widget|RemovefromParent _uicharacterdetailwidget))

(fn ConnecttoGame
  (Class|OWSPlayerControllerComponent|SetSelectedCharacterandConnecttoLastZone (Variables|Default|GetOWSPlayerControllerComponent) (Variables|Default|GetUserSessionGUID) (Variables|Default|GetCharacterName))
  (Dialogs|ShowLoadingDialog))

(fn Logout
  (Dialogs|HideCharacterDetailDialog)
  (Dialogs|ShowLoginDialog))

(fn CreateHubWorldCharacter
  (params (CharacterName :type String))
  (Class|OWSPlayerControllerComponent|CreateCharacterUsingDefaultCharacterValues (Variables|Default|GetOWSPlayerControllerComponent) (Variables|Default|GetUserSessionGUID) CharacterName "Default")
  (Variables|Default|SetCharacterName CharacterName))