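; Interactable supply pod that shows its open or closed state by swapping a material on the pod mesh.
; Interact checks whether the pod is already open and, if not, fires the opened event.
; The opened event applies a plain solid material and the closed event a blue one.
; All three events act only on the Remote branch of the authority switch, so this Blueprint's logic runs only without authority.
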(event EventBeginPlay)

(event Collision|EventActorBeginOverlap
  (params (OtherActor :type Actor%20Object%20Reference)))

(event EventTick
  (params (DeltaSeconds :type Float%20%28single-precision%29)))

(event EventSupplyPodOpened
  ;[1 1 1] When the Supply Pod is Opened or Closed, then Change the Material
  (Networking|SwitchHasAuthority
    (:Remote
      (Rendering|Material|SetMaterial (Variables|Default|GetClosedSupplyPod) 2 "/Game/_HWAssets/LevelPrototyping/Materials/M_Solid.M_Solid"))))

(event EventSupplyPodClosed
  ;[1 1 1] When the Supply Pod is Opened or Closed, then Change the Material
  (Networking|SwitchHasAuthority
    (:Remote
      (Rendering|Material|SetMaterial (Variables|Default|GetClosedSupplyPod) 2 "/Game/_HWAssets/LevelPrototyping/Materials/MI_Solid_Blue.MI_Solid_Blue"))))

(event EventInteract
  ;[1 1 1] On Interact - If the Supply Pod is Closed, then Open it
  (Networking|SwitchHasAuthority
    (:Remote
      (bind _returnvalue (Class|SupplyPod|IsSupplyPodOpened))
      (if (not _returnvalue)
        (Class|SupplyPod|SupplyPodOpened)))))

(fn ConstructionScript)